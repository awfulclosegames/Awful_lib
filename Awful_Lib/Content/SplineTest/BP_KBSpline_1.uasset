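; Test actor that builds and debug-draws KB splines from five point components, with a bounded constraint on one segment.
; BeginPlay fills two identical configs, adds the constraint between Point1 and Point2, and prepares evaluation states for three point IDs.
; AddBounds derives anchor bounds from the segment direction and its horizontal perpendicular, using tunable offsets.
; Tick draws the three states on the first spline; the second is never evaluated.
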(event `self.ReceiveBeginPlay`
  (bind _returnvalue (`self.K2_GetActorLocation`))
  (`|ExecutionSequence`
    (:`then_0`
      (bind _returnvalue_2 (`AC_KBSpline.CreateSplineConfig` _returnvalue))
      (set `self.Spline` _returnvalue_2)
      (bind _returnvalue_3 (`AC_KBSpline.CreateSplineConfig` _returnvalue))
      (set `self.Spline2` _returnvalue_3))
    (:`then_1`
      (`self.AddSplinePoint` (`self.Point 0`))
      (`self.AddSplinePoint` (`self.Point 1`))
      (`self.AddSplinePoint` (`self.Point 2`))
      (`self.AddSplinePoint` (`self.Point 3`))
      (`self.AddSplinePoint` (`self.Point 4`)))
    (:`then_2`
      (`self.AddBounds` (`SceneComponent.K2_GetComponentLocation` (`self.Point 1`)) (`SceneComponent.K2_GetComponentLocation` (`self.Point 2`)) 2))
    (:`then_3`
      (bind _returnvalue_4 (`AC_KBSpline.PrepareForEvaluation` (`self.Spline`)))
      (set `self.State1` _returnvalue_4)
      (bind _returnvalue_5 (`AC_KBSpline.PrepareForEvaluation` (`self.Spline`) 2))
      (set `self.State2` _returnvalue_5)
      (bind _returnvalue_6 (`AC_KBSpline.PrepareForEvaluation` (`self.Spline`) 3))
      (set `self.State3` _returnvalue_6))))

(event `self.ReceiveTick`
  (params (DeltaSeconds :type "Float (single-precision)"))
  (`AC_KBSpline.DrawDebug` self (`self.Spline`) (`self.State1`) (struct :`B` 255 :`A` 255))
  (`AC_KBSpline.DrawDebug` self (`self.Spline`) (`self.State2`) (struct :`B` 255 :`A` 255))
  (`AC_KBSpline.DrawDebug` self (`self.Spline`) (`self.State3`) (struct :`B` 255 :`A` 255)))

(fn `AddBounds`
  (params (From :type "Vector Structure") (To :type "Vector Structure") (SegmentID :type Integer))
  (bind _returnvalue (`KismetMathLibrary.Normal` (- To From)))
  (bind _returnvalue_2 (`KismetMathLibrary.Cross_VectorVector` _returnvalue (0.0 0.0 -1.0)))
  (bind _kbsplinebounds (make `KBSplineBounds` (`|MakeArray` (make `KBAnchorPoint` (make `KBSplinePoint` From) (+ (+ (* _returnvalue -12.0) (* _returnvalue_2 (`self.BoundsFMin`))) From) (+ (+ (* _returnvalue -10.0) (* _returnvalue_2 (`self.BoundsFMax`))) From)) (make `KBAnchorPoint` (make `KBSplinePoint` To) (+ (+ (* _returnvalue 10.0) (* _returnvalue_2 (`self.BoundsTMin`))) To) (+ (+ (* _returnvalue 10.0) (* _returnvalue_2 (`self.BoundsTMax`))) To)))))
  (`AC_KBSpline.AddSegmentConstraint` (`self.Spline`) _kbsplinebounds SegmentID)
  (`AC_KBSpline.AddSegmentConstraint` (`self.Spline2`) _kbsplinebounds SegmentID))

(fn `AddSplinePoint`
  (params (self2 :type "SceneComponent Object Reference"))
  (bind _kbsplinepoint (make `KBSplinePoint` (`SceneComponent.K2_GetComponentLocation` self2) -2.0))
  (`self.NewFunction` (`self.Spline`) _kbsplinepoint)
  (`self.NewFunction` (`self.Spline2`) _kbsplinepoint))

(fn `NewFunction`
  (params (Config :type "KBSplineConfig Object Reference") (Point :type "KBSplinePoint Structure"))
  (`AC_KBSpline.AddSplinePoint` Config Point))

(fn `UserConstructionScript`)