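; BP_KBSpline_1 is a test actor that builds a KB spline from five point components and draws it for debugging.
; On BeginPlay it creates the spline config at the actor location, adds each component's world location with shared tau and beta, then prepares three evaluation states for consecutive interior point IDs.
; Tick debug-draws those cached states every frame, without rebuilding the spline.
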(event `self.ReceiveBeginPlay`
  (`|ExecutionSequence`
    (:`then_0`
      (bind _returnvalue (`SDZ_KBSpline.CreateSplineConfig` (`self.K2_GetActorLocation`)))
      (set `self.Spline` _returnvalue))
    (:`then_1`
      (`self.AddSplinePoint` (`self.Point 0`))
      (`self.AddSplinePoint` (`self.Point 1`))
      (`self.AddSplinePoint` (`self.Point 2`))
      (`self.AddSplinePoint` (`self.Point 3`))
      (`self.AddSplinePoint` (`self.Point 4`)))
    (:`then_2`
      (bind _returnvalue_2 (`SDZ_KBSpline.PrepareForEvaluation` (`self.Spline`)))
      (set `self.State` _returnvalue_2)
      (bind _returnvalue_3 (`SDZ_KBSpline.PrepareForEvaluation` (`self.Spline`) 2))
      (set `self.Segment2` _returnvalue_3)
      (bind _returnvalue_4 (`SDZ_KBSpline.PrepareForEvaluation` (`self.Spline`) 3))
      (set `self.Segment3` _returnvalue_4))))

(event `self.ReceiveTick`
  (params (DeltaSeconds :type "Float (single-precision)"))
  (`SDZ_KBSpline.DrawDebug` self (`self.Spline`) (`self.State`))
  (`SDZ_KBSpline.DrawDebug` self (`self.Spline`) (`self.Segment2`))
  (`SDZ_KBSpline.DrawDebug` self (`self.Spline`) (`self.Segment3`)))

(fn `AddSplinePoint`
  (params (self2 :type "SceneComponent Object Reference"))
  (`self.NewFunction` (`self.Spline`) (make `KBSplinePoint` (`SceneComponent.K2_GetComponentLocation` self2) -1.0 0.0)))

(fn `NewFunction`
  (params (Config :type "KBSplineConfig Object Reference") (Point :type "KBSplinePoint Structure"))
  (`SDZ_KBSpline.AddSplinePoint` Config Point))

(fn `UserConstructionScript`)